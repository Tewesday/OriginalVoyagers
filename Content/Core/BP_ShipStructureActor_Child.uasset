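; BP_ShipStructureActor_Child is a ship structure actor that replaces itself with a BP_ShipUnitPawn_Child when play runs.
; On its first Tick, after the parent Tick, a DoOnce spawns the pawn at the actor's transform, ignoring collisions, then destroys the actor.
; The construction script only calls the parent, and the BeginPlay and overlap events are disabled stubs.
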(event `self.ReceiveTick`
  (params (DeltaSeconds :type "Float (single-precision)"))
  (`parent.ReceiveTick` DeltaSeconds)
  (`/Engine/EditorBlueprintResources/StandardMacros.DoOnce` false
    (:`Completed`
      (`|SpawnActorFromClass` "/Game/Core/BP_ShipUnitPawn_Child.BP_ShipUnitPawn_Child_C" (`self.GetTransform`) "AlwaysSpawn" "OverrideRootScale" null null)
      (`self.K2_DestroyActor`))))

(fn `UserConstructionScript`
  (`parent.UserConstructionScript`))