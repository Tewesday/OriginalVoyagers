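; BP_RegionPawn represents a named map region that owns structures and pays for them from its own resources.
; Overlaps on its RegionCollision keep sets of contained structures and neighboring region pawns, stamping each entering structure with the region's name as owner.
; Helper functions check structure affordability and deduct costs through the ResourceManagementSubsystem, both using the same fixed entry in its resource name list.
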(event `self.RegionCollision.OnComponentBeginOverlap`
  (params (OverlappedComponent :type "PrimitiveComponent Object Reference") (OtherActor :type "Actor Object Reference") (OtherComp :type "PrimitiveComponent Object Reference") (OtherBodyIndex :type Integer) (bFromSweep :type Boolean) (SweepResult :type "HitResult Structure (by ref)"))
  (`|ExecutionSequence`
    (:`then_0`
      ;[1 1 1] Assign owning region to structure and add to set
      (if (`KismetMathLibrary.ClassIsChildOf` (`GameplayStatics.GetObjectClass` OtherActor) "/Script/SeafaringPrototype.StructureActor")
        (bind _asbp_structure_actor (cast `/Game/Core/BP_StructureActor` OtherActor))
        (set `StructureActor.OwningRegion` (`self.RegionName`) _asbp_structure_actor)
        (`BlueprintSetLibrary.Set_Add` (`self.StructuresInRegion`) _asbp_structure_actor)))
    (:`then_1`
      ;[1 1 1] Add region to set
      (if (`KismetMathLibrary.ClassIsChildOf` (`GameplayStatics.GetObjectClass` OtherActor) "BP_RegionPawn_C")
        (bind _asbp_region_pawn (cast `/Game/Core/BP_RegionPawn` OtherActor))
        (`BlueprintSetLibrary.Set_Add` (`self.NearbyRegions`) _asbp_region_pawn)))))

(event `self.RegionCollision.OnComponentEndOverlap`
  (params (OverlappedComponent :type "PrimitiveComponent Object Reference") (OtherActor :type "Actor Object Reference") (OtherComp :type "PrimitiveComponent Object Reference") (OtherBodyIndex :type Integer))
  (`|ExecutionSequence`
    (:`then_0`
      ;[1 1 1] Remove structure from set
      (if (`KismetMathLibrary.ClassIsChildOf` (`GameplayStatics.GetObjectClass` OtherActor) "/Script/SeafaringPrototype.StructureActor")
        (bind _asbp_structure_actor (cast `/Game/Core/BP_StructureActor` OtherActor))
        (`BlueprintSetLibrary.Set_Remove` (`self.StructuresInRegion`) _asbp_structure_actor)))
    (:`then_1`
      ;[1 1 1] Remove region from set
      (if (`KismetMathLibrary.ClassIsChildOf` (`GameplayStatics.GetObjectClass` OtherActor) "BP_RegionPawn_C")
        (bind _asbp_region_pawn (cast `/Game/Core/BP_RegionPawn` OtherActor))
        (`BlueprintSetLibrary.Set_Remove` (`self.NearbyRegions`) _asbp_region_pawn)))))

(fn `CheckStructureAffordability`
  (params (StructureType :type String))
  (returns (StructureAffordable :type Boolean))
  (bind _returnvalue (subsystem `ResourceManagementSubsystem`))
  (bind _returnvalue_2 (`ResourceManagementSubsystem.RetrieveStructureCost` _returnvalue StructureType))
  (bind _returnvalue_3 (`ResourceManagementSubsystem.RetrieveResourceValue` _returnvalue (`self.RegionName`) (`|GetArrayItem` (`ResourceManagementSubsystem.ResourceNames` _returnvalue) 1)))
  (return (>= _returnvalue_3 _returnvalue_2)))

(fn `SpendResourcesOnStructure`
  (params (StructureCost :type Integer))
  (bind _returnvalue (subsystem `ResourceManagementSubsystem`))
  (`ResourceManagementSubsystem.DecrementResourceByAmount` _returnvalue (`self.RegionName`) (`|GetArrayItem` (`ResourceManagementSubsystem.ResourceNames` _returnvalue) 1) StructureCost))

(fn `UserConstructionScript`)