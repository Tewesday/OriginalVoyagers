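; BP_PopulationStructureActor_Child is a population structure that periodically grows its owning region's population and spawns units.
; BeginPlay starts a looping timer on AddPopulation, which increments the default population through the PopulationSubsystem and prints the result.
; Each cycle also spawns a BP_UnitPawn offset along negative world X from the structure, ignoring collision.
; Tick clears the timer once the actor is being destroyed.
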(event `self.ReceiveBeginPlay`
  (`parent.ReceiveBeginPlay`)
  (`KismetSystemLibrary.K2_SetTimer` null "AddPopulation" 5.0 true))

(event `self.ReceiveTick`
  (params (DeltaSeconds :type "Float (single-precision)"))
  (`parent.ReceiveTick` DeltaSeconds)
  (if (`self.IsActorBeingDestroyed`)
    (`KismetSystemLibrary.K2_ClearTimer` null "AddPopulation")))

(fn `AddPopulation`
  (locals (ActorSpawnDisplacement :type "Float (double-precision)" :default 20.0))
  (bind _owningregion (`self.OwningRegion`))
  (bind _returnvalue (`PopulationSubsystem.IncrementPopulation` (subsystem `PopulationSubsystem`) _owningregion (`self.PopulationNameDefault`)))
  (`KismetSystemLibrary.PrintString` (`KismetStringLibrary.Concat_StrStr` (`KismetStringLibrary.Concat_StrStr` (`KismetStringLibrary.Conv_IntToString` _returnvalue) " population added to ") _owningregion))
  (`|SpawnActorFromClass` "/Game/Core/BP_UnitPawn.BP_UnitPawn_C" (`KismetMathLibrary.MakeTransform` (`KismetMathLibrary.MakeVector` (- (.x (.location (`self.GetTransform`))) (`local.ActorSpawnDisplacement`)) (.y (.location (`self.GetTransform`))) (.z (.location (`self.GetTransform`)))) (.rotation (`self.GetTransform`)) (.scale (`self.GetTransform`))) "AlwaysSpawn" "OverrideRootScale" null null))

(fn `UserConstructionScript`
  (`parent.UserConstructionScript`))