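; Main gameplay HUD for a region-based strategy game, creating resource, transfer, structure and win/loss widgets.
; DrawHUD runs gated drag box-selection of BasicPawns into UnitManagementSubsystem and spawns nav point markers from queued points.
; Left-click release places structures via a cursor trace that rejects overlaps, finds the region, checks affordability and spends its resources.
; Update functions fill region resources, population and nearby-region dropdown from subsystems and the level manager.
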(event `self.ReceiveBeginPlay`
  (`self.EnableInput` (`GameplayStatics.GetPlayerController` 0))
  (bind _returnvalue (`|CreateWidget` "/Game/Core/BP_RegionResourcesWidget.BP_RegionResourcesWidget_C" (`GameplayStatics.GetPlayerController` 0)))
  (set `self.ResourcesWidget` _returnvalue)
  (`UserWidget.AddToViewport` _returnvalue 0)
  (`Widget.SetRenderTransform` _returnvalue (make `WidgetTransform` (748.0 0.0)))
  (bind _returnvalue_2 (`|CreateWidget` "/Game/Core/BP_RegionResourceTransferWidget.BP_RegionResourceTransferWidget_C" (`GameplayStatics.GetPlayerController` 0)))
  (set `self.ResourceTransferWidget` _returnvalue_2)
  (`UserWidget.AddToViewport` _returnvalue_2 0)
  (`Widget.SetRenderTransform` _returnvalue_2 (make `WidgetTransform` (0.0 0.0)))
  ;[1 1 1] Set reference to LevelManager
  (bind _outactors (`GameplayStatics.GetAllActorsOfClass` "/Game/Core/BP_LevelManager.BP_LevelManager_C"))
  (for _array_element _outactors
    (bind _asbp_level_manager (cast `/Game/Core/BP_LevelManager` _array_element))
    (set `self.LevelManagerRef` _asbp_level_manager)
    (break))
  (bind _returnvalue_3 (`|CreateWidget` "/Game/Core/BP_StructureWidget.BP_StructureWidget_C" (`GameplayStatics.GetPlayerController` 0)))
  (set `/Game/Core/BP_StructureWidget.StructureType` "WoodCollector" _returnvalue_3)
  (`UserWidget.AddToViewport` _returnvalue_3 0)
  (bind _returnvalue_4 (`|CreateWidget` "/Game/Core/BP_FoodStructureWidget1.BP_FoodStructureWidget1_C" (`GameplayStatics.GetPlayerController` 0)))
  (set `/Game/Core/BP_FoodStructureWidget1.StructureType` "FoodCollector" _returnvalue_4)
  (`UserWidget.AddToViewport` _returnvalue_4 0)
  (`Widget.SetRenderTransform` _returnvalue_4 (make `WidgetTransform` (172.0 0.0)))
  (bind _returnvalue_5 (`|CreateWidget` "/Game/Core/BP_PopulationStructureWidget.BP_PopulationStructureWidget_C" (`GameplayStatics.GetPlayerController` 0)))
  (set `/Game/Core/BP_PopulationStructureWidget.StructureType` "CultureCollector" _returnvalue_5)
  (`UserWidget.AddToViewport` _returnvalue_5 0)
  (`Widget.SetRenderTransform` _returnvalue_5 (make `WidgetTransform` (336.0 0.0)))
  (bind _returnvalue_6 (`|CreateWidget` "/Game/Core/BP_ShipStructureWidget.BP_ShipStructureWidget_C" (`GameplayStatics.GetPlayerController` 0)))
  (set `/Game/Core/BP_ShipStructureWidget.StructureType` "Ship" _returnvalue_6)
  (`UserWidget.AddToViewport` _returnvalue_6 0)
  (`Widget.SetRenderTransform` _returnvalue_6 (make `WidgetTransform` (508.0 0.0))))

(event `self.ReceiveDrawHUD`
  (params (SizeX :type Integer) (SizeY :type Integer))
  (bind _drawpoints (`self.DrawPoints`))
  (bind (_locationx _locationy) (`PlayerController.GetMousePosition` (`GameplayStatics.GetPlayerController` 0)))
  (bind _returnvalue (`KismetMathLibrary.MakeVector2D` _locationx _locationy))
  (`|ExecutionSequence`
    (:`then_0`
      ;[1 1 1] Box Select
      (`/Engine/EditorBlueprintResources/StandardMacros.Gate` true :!label _label
        (:`Exit`
          (`UnitManagementSubsystem.RemoveSelection` (pcsubsystem `UnitManagementSubsystem` (`GameplayStatics.GetPlayerController` 0)))
          (`KismetArrayLibrary.Array_Clear` (`self.Selection to Add`))
          (if (`self.BoxComplete`)
            (bind (_x _y) (`KismetMathLibrary.BreakVector2D` (stale `InputAction|LeftClick` _output_get)))
            (bind (_x_2 _y_2) (`KismetMathLibrary.BreakVector2D` (- _returnvalue (stale `InputAction|LeftClick` _output_get))))
            (`self.DrawRect` (struct :`G` 0.392 :`A` 0.4) _x _y _x_2 _y_2)
            (else
              (for _array_element (`self.GetActorsInSelectionRectangle` "/Script/SeafaringPrototype.BasicPawn" (`self.StartPoint`) _returnvalue)
                (bind _asbasic_pawn (cast `BasicPawn` _array_element))
                (`KismetArrayLibrary.Array_Add` (`self.Selection to Add`) _asbasic_pawn)
                (`KismetSystemLibrary.PrintString` (`KismetSystemLibrary.GetDisplayName` _array_element))
                (set `self.BoxComplete` true :!label _label_2)
                (goto _label :!via `Close`))
              (`UnitManagementSubsystem.AddSelection` (pcsubsystem `UnitManagementSubsystem` (`GameplayStatics.GetPlayerController` 0)) (`self.Selection to Add`))
              (goto _label_2))))))
    (:`then_1`
      (if (>= (`KismetArrayLibrary.Array_Length` _drawpoints) 1)
        (bind _returnvalue_2 (`|SpawnActorFromClass` "/Game/Core/BP_NavPoint.BP_NavPoint_C" (`KismetMathLibrary.MakeTransform` (`|GetArrayItem` _drawpoints)) "Undefined" "OverrideRootScale" null null))
        (`KismetArrayLibrary.Array_Add` (`self.PathPoints`) _returnvalue_2)
        (`KismetArrayLibrary.Array_Clear` (`self.DrawPoints`))))))

(event `InputAction|LeftClick`
  (params (Key :type "Key Structure"))
  (bind (_locationx _locationy) (`PlayerController.GetMousePosition` (`GameplayStatics.GetPlayerController` 0)))
  (:`Pressed`
    (if (`self.BoxSelectEnabled`)
      ;[1 1 1] Box Select
      (bind _output_get (set `self.StartPoint` (`KismetMathLibrary.MakeVector2D` _locationx _locationy)))
      (goto _label :!via `Open`)))
  (:`Released`
    (`|ExecutionSequence`
      (:`then_0`
        (if (`self.BoxSelectEnabled`)
          (set `self.BoxComplete` false)))
      (:`then_1`
        ;[1 1 1] Place structure
        (if (`self.PlacingStructure`)
          (`self.PlaceStructure`)
          (set `self.PlacingStructure` false)
          (set `self.BoxSelectEnabled` true)
          (`KismetSystemLibrary.PrintString` "Structure placed"))))))

(fn `ClearPathPoints`
  (for _array_element (`self.PathPoints`)
    (`self.K2_DestroyActor` _array_element))
  (`KismetArrayLibrary.Array_Clear` (`self.PathPoints`)))

(fn `DisplayLoss`
  (bind _returnvalue (`|CreateWidget` "/Game/Core/BP_LossWidget.BP_LossWidget_C" (`GameplayStatics.GetPlayerController` 0)))
  (`UserWidget.AddToViewport` _returnvalue 0)
  (`Widget.SetRenderTransform` _returnvalue (make `WidgetTransform` (0.0 0.0))))

(fn `DisplayWin`
  (bind _returnvalue (`|CreateWidget` "/Game/Core/BP_WinWidget.BP_WinWidget_C" (`GameplayStatics.GetPlayerController` 0)))
  (`UserWidget.AddToViewport` _returnvalue 0)
  (`Widget.SetRenderTransform` _returnvalue (make `WidgetTransform` (0.0 0.0))))

(fn `DrawPersistingRectangle`
  (params (FirstPoint :type "Vector2D Structure") (SecondPoint :type "Vector2D Structure"))
  (locals (FirstPointVar :type "Vector2D Structure") (SecondPointVar :type "Vector2D Structure"))
  (bind (_x _y) (`KismetMathLibrary.BreakVector2D` (`local.FirstPointVar`)))
  (bind _output_get (set `local.FirstPointVar` FirstPoint))
  (bind _output_get_2 (set `local.SecondPointVar` SecondPoint))
  (bind (_x_2 _y_2) (`KismetMathLibrary.BreakVector2D` (- _output_get_2 _output_get)))
  (`self.DrawRect` (struct :`G` 0.392 :`A` 0.4) _x _y _x_2 _y_2))

(fn `GetStructureClassFromStructureType`
  (params (StructureType :type String))
  (returns (ClassType :type "/Game/Core/BP_StructureActor Class Reference"))
  (for _array_element (`/Game/Core/BP_LevelManager.PossibleStructures` (`self.LevelManagerRef`))
    (if (`KismetStringLibrary.EqualEqual_StrStr` StructureType (`.DefaultStructureType` (defaults `Object` _array_element)))
      (return _array_element))))

(fn `GiveNewDrawPoint`
  (params (NewPoint :type "Vector Structure"))
  (`KismetArrayLibrary.Array_Add` (`self.DrawPoints`) NewPoint))

(fn `PlaceStructure`
  (bind _currentlyselectedstructuretype (`self.CurrentlySelectedStructureType`))
  (bind (_worldlocation _worlddirection) (`PlayerController.DeprojectMousePositionToWorld` (`GameplayStatics.GetPlayerController` 0)))
  (bind _returnvalue (`KismetMathLibrary.MakeVector` (.x (+ _worldlocation (* _worlddirection (`self.MouseZAccuracy`)))) (.y (+ _worldlocation (* _worlddirection (`self.MouseZAccuracy`))))))
  ;[1 1 1] Verify that structure can be placed (not overlapping structure)
  (bind _outhits (`KismetSystemLibrary.LineTraceMultiForObjects` :`Start` _worldlocation :`End` _returnvalue :`ObjectTypes` (`self.Object Types`) :`DrawDebugType` "ForOneFrame"))
  (for _array_element _outhits
    (`|ExecutionSequence`
      (:`then_0`
        (bind (_bblockinghit _binitialoverlap _time _distance _location _impactpoint _normal _impactnormal _physmat _hitactor) (`GameplayStatics.BreakHitResult` _array_element))
        (bind _returnvalue_2 (`GameplayStatics.GetObjectClass` _hitactor))
        (if (`KismetMathLibrary.ClassIsChildOf` _returnvalue_2 "/Game/Core/BP_StructureActor.BP_StructureActor_C")
          (set `self.StructurePlacementValid` false)))
      (:`then_1`
        (if (`KismetMathLibrary.ClassIsChildOf` _returnvalue_2 "/Script/SeafaringPrototype.RegionPawn")
          (bind _asbp_region_pawn (cast `/Game/Core/BP_RegionPawn` _hitactor))
          (set `self.RegionNameForStructure` (`RegionPawn.RegionName` _asbp_region_pawn))))))
  (if (`self.StructurePlacementValid`)
    (bind _regionchosen (`/Game/Core/BP_LevelManager.GetRegionUsingName` (`self.LevelManagerRef`) (`self.RegionNameForStructure`)))
    (if (`KismetSystemLibrary.IsValid` _regionchosen)
      (bind _structureaffordable (`/Game/Core/BP_RegionPawn.CheckStructureAffordability` _regionchosen _currentlyselectedstructuretype))
      (set `self.PlayerCanAffordStructure` _structureaffordable)
      (if (`self.PlayerCanAffordStructure`)
        (bind _returnvalue_3 (`ResourceManagementSubsystem.RetrieveStructureCost` (subsystem `ResourceManagementSubsystem`) _currentlyselectedstructuretype))
        (`/Game/Core/BP_RegionPawn.SpendResourcesOnStructure` _regionchosen _returnvalue_3)
        (bind _classtype (`self.GetStructureClassFromStructureType` (`self.CurrentlySelectedStructureType`)))
        (`|SpawnActorFromClass` _classtype (`KismetMathLibrary.MakeTransform` _returnvalue) "AlwaysSpawn" "OverrideRootScale" null null)
        (set `self.BoxSelectEnabled` true)
        (set `self.StructurePlacementValid` true))
      (else
        (set `self.BoxSelectEnabled` true)
        (set `self.StructurePlacementValid` true)))
    (else
      (`KismetSystemLibrary.PrintString` "Structures cannot overlap")
      (set `self.BoxSelectEnabled` true)
      (set `self.StructurePlacementValid` true))))

(fn `UpdateNearbyRegions`
  (bind _levelmanagerref (`self.LevelManagerRef`))
  (bind _currentlyselectedregion (`/Game/Core/BP_LevelManager.CurrentlySelectedRegion` _levelmanagerref))
  (`ComboBoxString.ClearOptions` (`/Game/Core/BP_RegionResourceTransferWidget.NearbyRegionsDropdown` (`self.ResourceTransferWidget`)))
  (if (`KismetStringLibrary.NotEqual_StrStr` _currentlyselectedregion)
    (bind _regionchosen (`/Game/Core/BP_LevelManager.GetRegionUsingName` _levelmanagerref _currentlyselectedregion))
    (bind _nearbyregions (`/Game/Core/BP_RegionPawn.NearbyRegions` _regionchosen))
    (if (> (`BlueprintSetLibrary.Set_Length` _nearbyregions) 0)
      (bind _result (`BlueprintSetLibrary.Set_ToArray` _nearbyregions))
      (for _array_element _result
        (`ComboBoxString.AddOption` (`/Game/Core/BP_RegionResourceTransferWidget.NearbyRegionsDropdown` (`self.ResourceTransferWidget`)) (`RegionPawn.RegionName` _array_element))))))

(fn `UpdatePopulation`
  (params (Region :type String))
  (bind _returnvalue (`PopulationSubsystem.RetrievePopulationValue` (subsystem `PopulationSubsystem`) Region (`/Game/Core/BP_LevelManager.PopulationNameDefault` (`self.LevelManagerRef`))))
  (bind _returnvalue_2 (`KismetTextLibrary.Conv_IntToText` _returnvalue))
  (`EditableText.SetText` (`/Game/Core/BP_RegionResourcesWidget.ExtraText` (`self.ResourcesWidget`)) _returnvalue_2)
  (`EditableText.SetText` (`/Game/Core/BP_RegionResourceTransferWidget.CurrentRegionPopulationText` (`self.ResourceTransferWidget`)) _returnvalue_2))

(fn `UpdateResources`
  (params (Region :type String))
  (bind _returnvalue (`KismetTextLibrary.Conv_StringToText` Region))
  (bind _returnvalue_2 (subsystem `ResourceManagementSubsystem`))
  (bind _resourceswidget (`self.ResourcesWidget`))
  (bind _resourcetransferwidget (`self.ResourceTransferWidget`))
  (`EditableText.SetText` (`/Game/Core/BP_RegionResourcesWidget.ResourcesText` (`self.ResourcesWidget`)) _returnvalue)
  (`EditableText.SetText` (`/Game/Core/BP_RegionResourceTransferWidget.CurrentRegionText` (`self.ResourceTransferWidget`)) _returnvalue)
  (for (_array_element _array_index) (`ResourceManagementSubsystem.ResourceNames` _returnvalue_2)
    (bind _returnvalue_3 (`ResourceManagementSubsystem.RetrieveResourceValue` _returnvalue_2 Region _array_element))
    (switch `int` _array_index
      (:`0`
        (bind _returnvalue_4 (`KismetTextLibrary.Conv_IntToText` _returnvalue_3))
        (`EditableText.SetText` (`/Game/Core/BP_RegionResourcesWidget.FoodText` _resourceswidget) _returnvalue_4)
        (`EditableText.SetText` (`/Game/Core/BP_RegionResourceTransferWidget.CurrentRegionFoodText` _resourcetransferwidget) _returnvalue_4))
      (:`1`
        (`EditableText.SetText` (`/Game/Core/BP_RegionResourcesWidget.WoodText` _resourceswidget) _returnvalue_4)
        (`EditableText.SetText` (`/Game/Core/BP_RegionResourceTransferWidget.CurrentRegionWoodText` _resourcetransferwidget) _returnvalue_4))))
  (`|ExecutionSequence`
    (:`then_0`
      (bind _regionchosen (`/Game/Core/BP_LevelManager.GetRegionUsingName` (`self.LevelManagerRef`) Region))
      (`EditableText.SetText` (`/Game/Core/BP_RegionResourceTransferWidget.CurrentRegionMaxWeightText` (`self.ResourceTransferWidget`)) (`KismetTextLibrary.Conv_IntToText` (`/Game/Core/BP_RegionPawn.RegionMaxWeight` _regionchosen))))
    (:`then_1`
      (`self.UpdatePopulation` Region))
    (:`then_2`
      (`self.UpdateNearbyRegions`))))

(fn `UserConstructionScript`)