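; Player controller for a top-down strategy game, handling camera panning, drawn unit paths and region selection.
; Holding right click samples deprojected cursor points on a timer and previews them on the HUD.
; Release turns the points into a BP_BasicRail spline, which UnitManagementSubsystem assigns to units.
; A repeating downward trace from the pawn sets the level manager's selected BP_RegionPawn region and refreshes HUD resources.
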(event `self.ReceiveBeginPlay`
  (`KismetSystemLibrary.K2_SetTimer` null "TraceForCurrentRegion" 1.0)
  (`KismetSystemLibrary.K2_SetTimer` null "UpdateTraceFrequency" 2.5))

(event `InputAction|RightClick`
  (params (Key :type "Key Structure"))
  (bind _setoflocations (`self.SetOfLocations`))
  (bind _returnvalue (pcsubsystem `UnitManagementSubsystem` self))
  (:`Pressed`
    (`/Engine/EditorBlueprintResources/StandardMacros.DoOnce` false :!label _label
      (:`Completed`
        (if (`KismetSystemLibrary.IsValid` (`self.CurrentRail`))
          (`self.K2_DestroyActor`)
          (set `self.CurrentRail` null)
          (set `self.RailSpawned` false))
        (bind _returnvalue_2 (`KismetSystemLibrary.K2_SetTimer` null "AddLocation" 0.05 true)))))
  (:`Released`
    (`KismetSystemLibrary.K2_ClearAndInvalidateTimerHandle` _returnvalue_2)
    (bind _asbp_basic_hud (cast `/Game/UI/BP_BasicHUD` (`self.GetHUD`)))
    (`/Game/UI/BP_BasicHUD.ClearPathPoints` _asbp_basic_hud)
    (for _array_element _setoflocations
      (if (`self.RailSpawned`)
        (`/Game/Core/BP_BasicRail.AddNewSplinePointOnEnd` (`self.CurrentRail`) _array_element)
        (else
          (bind _returnvalue_3 (`|SpawnActorFromClass` "/Game/Core/BP_BasicRail.BP_BasicRail_C" (`KismetMathLibrary.MakeTransform` _array_element) "Undefined" "OverrideRootScale" null null))
          (bind _output_get (set `self.CurrentRail` _returnvalue_3))
          (set `self.RailSpawned` true)
          (`UnitManagementSubsystem.AssignPathToUnits` _returnvalue _output_get)
          (`UnitManagementSubsystem.InstructUnits` _returnvalue))))
    (`KismetArrayLibrary.Array_Clear` _setoflocations)
    (goto _label :!via `Reset`)))

(event `InputAxis|ForwardMovement`
  (params (AxisValue :type "Float (single-precision)"))
  (bind _rootcomponent (`Actor.RootComponent` (`GameplayStatics.GetPlayerPawn` 0)))
  (bind (_returnvalue_x _returnvalue_y _returnvalue_z) (`KismetMathLibrary.BreakVector` (`SceneComponent.K2_GetComponentLocation` _rootcomponent)))
  (`SceneComponent.K2_SetWorldLocation` _rootcomponent (`KismetMathLibrary.MakeVector` (+ (* AxisValue (`self.CameraMoveSpeed`)) _returnvalue_x) _returnvalue_y _returnvalue_z) false false))

(event `InputAxis|SidewaysMovement`
  (params (AxisValue :type "Float (single-precision)"))
  (bind _rootcomponent (`Actor.RootComponent` (`GameplayStatics.GetPlayerPawn` 0)))
  (bind (_returnvalue_x _returnvalue_y _returnvalue_z) (`KismetMathLibrary.BreakVector` (`SceneComponent.K2_GetComponentLocation` _rootcomponent)))
  (`SceneComponent.K2_SetWorldLocation` _rootcomponent (`KismetMathLibrary.MakeVector` _returnvalue_x (+ (* AxisValue (`self.CameraMoveSpeed`)) _returnvalue_y) _returnvalue_z) false false))

(fn `AddLocation`
  (bind (_worldlocation _worlddirection) (`self.DeprojectMousePositionToWorld`))
  (bind _returnvalue (+ _worldlocation (* _worlddirection (`self.MouseZAccuracy`))))
  (bind _returnvalue_2 (`KismetMathLibrary.MakeVector` (.x _returnvalue) (.y _returnvalue)))
  (`KismetSystemLibrary.PrintString` (`KismetStringLibrary.Conv_VectorToString` _returnvalue))
  (`KismetArrayLibrary.Array_Add` (`self.SetOfLocations`) _returnvalue_2)
  (bind _asbp_basic_hud (cast `/Game/UI/BP_BasicHUD` (`self.GetHUD`)))
  (`/Game/UI/BP_BasicHUD.GiveNewDrawPoint` _asbp_basic_hud _returnvalue_2))

(fn `GetLocation`
  (bind (_worldlocation _worlddirection) (`self.DeprojectMousePositionToWorld`))
  (bind _returnvalue (`KismetMathLibrary.MakeVector` (.x (+ _worldlocation (* _worlddirection 900.0))) (.y (+ _worldlocation (* _worlddirection 900.0)))))
  (if (!= _returnvalue (stale _output_get) :`ErrorTolerance` 1.0)
    (bind _output_get (set `self.LocationForSelect` _returnvalue))
    (`KismetSystemLibrary.PrintString` (`KismetStringLibrary.Conv_VectorToString` _output_get))
    (`self.LocationForSelectSet`)))

(fn `TraceForCurrentRegion`
  (bind (_returnvalue_x _returnvalue_y _returnvalue_z) (`KismetMathLibrary.BreakVector` (`SceneComponent.K2_GetComponentLocation` (`Actor.RootComponent` (`GameplayStatics.GetPlayerPawn` 0)))))
  (bind _outhits (`KismetSystemLibrary.LineTraceMulti` (`KismetMathLibrary.MakeVector` _returnvalue_x _returnvalue_y _returnvalue_z) (`KismetMathLibrary.MakeVector` _returnvalue_x _returnvalue_y) "TraceTypeQuery1"))
  (for _array_element _outhits
    (bind (_bblockinghit _binitialoverlap _time _distance _location _impactpoint _normal _impactnormal _physmat _hitactor) (`GameplayStatics.BreakHitResult` _array_element))
    (if (`KismetMathLibrary.ClassIsChildOf` (`GameplayStatics.GetObjectClass` _hitactor) "/Game/Core/BP_RegionPawn.BP_RegionPawn_C")
      (bind _asbp_region_pawn (cast `/Game/Core/BP_RegionPawn` _hitactor))
      (bind _outactors (`GameplayStatics.GetAllActorsOfClass` "/Game/Core/BP_LevelManager.BP_LevelManager_C"))
      (bind _output_get (set `/Game/Core/BP_LevelManager.CurrentlySelectedRegion` (`RegionPawn.RegionName` _asbp_region_pawn) (`|GetArrayItem` _outactors)))
      (bind _asbp_basic_hud (cast `/Game/UI/BP_BasicHUD` (`self.GetHUD`)))
      (`/Game/UI/BP_BasicHUD.UpdateResources` _asbp_basic_hud _output_get))))

(fn `UpdateTraceFrequency`
  (`KismetSystemLibrary.K2_SetTimer` null "TraceForCurrentRegion" 1.0 true))

(fn `UserConstructionScript`)