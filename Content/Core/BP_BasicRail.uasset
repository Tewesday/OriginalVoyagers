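; BP_BasicRail is a spline rail that tracks the progress of a mount moving along it.
; Reaching the beginning opens a Tick gate that advances a normalized position each frame, scaled by spline length to aim for consistent speed.
; At position 1.0 a second gate fires the end-of-rail event once, which closes the Tick gate.
; Helper functions append world-space spline points and set the StartSet flag.
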(event `self.ReceiveBeginPlay`
  (set `self.Rail Spline Component Ref` (`self.GetComponentByClass` "/Script/Engine.SplineComponent"))
  (add `self.BeginningOfRailReachedEvent` (delegate `BeginningReached`))
  (add `self.EndOfRailReachedEvent` (delegate `EndReached`)))

(event `BeginningReached`
  (bind _endofrailreached (`self.EndOfRailReached`))
  (goto _label :!via `Open`))

(event `self.ReceiveTick`
  (params (DeltaSeconds :type "Float (single-precision)"))
  (bind _endofrailreached (`self.EndOfRailReached`))
  (`/Engine/EditorBlueprintResources/StandardMacros.Gate` true :!label _label
    (:`Exit`
      ;[1 1 1] Move Mount along Rail
      (if _endofrailreached
        (`/Engine/EditorBlueprintResources/StandardMacros.Gate` true :!label _label_2
          (:`Exit`
            (`self.EndOfRailReachedEvent`)
            (goto _label_2 :!via `Close`)))
        (elif (not _endofrailreached)
          (bind _output_get (set `self.RailPosition` (+ (`KismetMathLibrary.NormalizeToRange` (`KismetMathLibrary.NormalizeToRange` (+ (`self.RailMoveSpeed`) (`self.RailPosition`)) 0.0 (`SplineComponent.GetSplineLength` (`self.Rail Spline Component Ref`))) 0.0 1.0) (`self.RailPosition`))))
          (bind _output_get_2 (set `self.CurrentPositionOnRail` _output_get))
          (set `self.EndOfRailReached` (>= _output_get_2 1.0))
          (goto _label_2 :!via `Open`))))))

(event `EndReached`
  (goto _label :!via `Close`))

(fn `AddNewSplinePointOnEnd`
  (params (Position :type "Vector Structure"))
  (`SplineComponent.AddSplinePoint` (`self.Rail Spline Component Ref`) Position "World" true))

(fn `SetStartSet`
  (params (SetTo :type Boolean))
  (set `self.StartSet` SetTo))

(fn `UserConstructionScript`)