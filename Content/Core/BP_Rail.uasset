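; Rail actor that tracks progress along a spline and signals when the end is reached.
; Tick adds raw delta time to the rail position until it reaches 1.0, then a gate fires the end-of-rail event once.
; AddNewSplinePointOnEnd extends the cached spline at a world location and adds a spline mesh component, without attaching or shaping it.
; The spline is never sampled here, so nothing moves along it.
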(event `self.ReceiveBeginPlay`
  (set `self.RailSplineComponentRef` (`self.GetComponentByClass` "/Script/Engine.SplineComponent")))

(event `self.ReceiveTick`
  (params (DeltaSeconds :type "Float (single-precision)"))
  (if (`self.EndOfRailReached`)
    (`/Engine/EditorBlueprintResources/StandardMacros.Gate` true :!label _label
      (:`Exit`
        (`self.EndOfRailReachedEvent`)
        (goto _label :!via `Close`)))
    (elif (not (`self.EndOfRailReached`))
      (bind _output_get (set `self.RailPosition` (+ DeltaSeconds (`self.RailPosition`))))
      (bind _output_get_2 (set `self.CurrentPositionOnRail` _output_get))
      (set `self.EndOfRailReached` (>= _output_get_2 1.0))
      (goto _label :!via `Open`))))

(fn `AddNewSplinePointOnEnd`
  (params (Location :type "Vector Structure"))
  (`SplineComponent.AddSplinePoint` (`self.RailSplineComponentRef`) Location "World" true)
  (`AddComponent|NODE_AddSplineMeshComponent-0` :`bManualAttachment` true))

(fn `UserConstructionScript`)