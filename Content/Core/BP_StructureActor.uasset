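; Base resource-gathering structure that harvests matching resource actors in range and credits the yield to its owning region; child classes override quality and resource type.
; Overlap spheres track nearby resources and assign unit pawns as workers, up to a cap.
; A looping timer drains each resource, reports the total to the resource management subsystem and destroys depleted actors.
; A backup region name guards against empty or "Voyager"-prefixed owners.
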(event `self.ReceiveBeginPlay`
  ;[1 1 1] Set default Quality and Resource Type, Should override values in child classes
  (set `self.StructureQuality` 1)
  (set `self.ResourceType` (`|GetArrayItem` (`ResourceManagementSubsystem.ResourceNames` (subsystem `ResourceManagementSubsystem`)) 1))
  (set `self.MaxWorkers` 5)
  (if (`KismetStringLibrary.NotEqual_StrStr` (`self.OwningRegion`))
    (`KismetSystemLibrary.K2_SetTimer` null "GatherResources" (`self.GatherRate`) true)))

(event `self.ReceiveActorBeginOverlap`
  (params (OtherActor :type "Actor Object Reference"))
  (bind _owningregion (`self.OwningRegion`))
  (if (`KismetStringLibrary.NotEqual_StrStr` _owningregion)
    (if (`KismetStringLibrary.StartsWith` (`self.OwningRegion`) "Voyager")
      (set `self.OwningRegion` (`self.BackupOfOwningRegion`))
      (else
        (set `self.BackupOfOwningRegion` _owningregion)
        (`/Engine/EditorBlueprintResources/StandardMacros.Gate` false :!label _label
          (:`Exit`
            (`/Engine/EditorBlueprintResources/StandardMacros.DoOnce` false
              (:`Completed`
                (`KismetSystemLibrary.K2_SetTimer` null "GatherResources" (`self.GatherRate`) true)
                (goto _label :!via `Close`)))))))))

(event `self.GatherRadiusCollision.OnComponentBeginOverlap`
  (params (OverlappedComponent :type "PrimitiveComponent Object Reference") (OtherActor :type "Actor Object Reference") (OtherComp :type "PrimitiveComponent Object Reference") (OtherBodyIndex :type Integer) (bFromSweep :type Boolean) (SweepResult :type "HitResult Structure (by ref)"))
  ;[1 1 1] Add resource of desired type to set of resources
  (if (`KismetMathLibrary.ClassIsChildOf` (`GameplayStatics.GetObjectClass` OtherActor) "/Script/SeafaringPrototype.ResourceActor")
    (bind _asresource_actor (cast `ResourceActor` OtherActor))
    (if (`KismetStringLibrary.EqualEqual_StrStr` (`ResourceActor.ResourceType` _asresource_actor) (`self.ResourceType`))
      (`BlueprintSetLibrary.Set_Add` (`self.ResourceActors`) _asresource_actor))))

(event `self.GatherRadiusCollision.OnComponentEndOverlap`
  (params (OverlappedComponent :type "PrimitiveComponent Object Reference") (OtherActor :type "Actor Object Reference") (OtherComp :type "PrimitiveComponent Object Reference") (OtherBodyIndex :type Integer))
  ;[1 1 1] Remove resource of desired type from set of resources
  (if (`KismetMathLibrary.ClassIsChildOf` (`GameplayStatics.GetObjectClass` OtherActor) "/Script/SeafaringPrototype.ResourceActor")
    (cast `ResourceActor` OtherActor)
    (`BlueprintSetLibrary.Set_Remove` (`self.ResourceActors`) OtherActor)))

(event `self.WorkerLoadRadiusCollision.OnComponentBeginOverlap`
  (params (OverlappedComponent :type "PrimitiveComponent Object Reference") (OtherActor :type "Actor Object Reference") (OtherComp :type "PrimitiveComponent Object Reference") (OtherBodyIndex :type Integer) (bFromSweep :type Boolean) (SweepResult :type "HitResult Structure (by ref)"))
  ;[1 1 1] Assign/Unassign Workers to building
  (if (`KismetMathLibrary.ClassIsChildOf` (`GameplayStatics.GetObjectClass` OtherActor) "/Game/Core/BP_UnitPawn.BP_UnitPawn_C")
    (bind _asbp_unit_pawn (cast `/Game/Core/BP_UnitPawn` OtherActor))
    (if (not (== (`self.MaxWorkers`) (`BlueprintSetLibrary.Set_Length` (`self.Workers`))))
      (`BlueprintSetLibrary.Set_Add` (`self.Workers`) _asbp_unit_pawn))))

(event `self.WorkerLoadRadiusCollision.OnComponentEndOverlap`
  (params (OverlappedComponent :type "PrimitiveComponent Object Reference") (OtherActor :type "Actor Object Reference") (OtherComp :type "PrimitiveComponent Object Reference") (OtherBodyIndex :type Integer))
  ;[1 1 1] Assign/Unassign Workers to building
  (if (`KismetMathLibrary.ClassIsChildOf` (`GameplayStatics.GetObjectClass` OtherActor) "/Game/Core/BP_UnitPawn.BP_UnitPawn_C")
    (bind _asbp_unit_pawn (cast `/Game/Core/BP_UnitPawn` OtherActor))
    (`BlueprintSetLibrary.Set_Remove` (`self.Workers`) _asbp_unit_pawn)))

(event `self.ReceiveDestroyed`
  (`KismetSystemLibrary.K2_ClearTimer` null "GatherResources"))

(fn `GatherResources`
  (bind _owningregion (`self.OwningRegion`))
  (bind _resourcetype (`self.ResourceType`))
  (if (`KismetStringLibrary.StartsWith` (`self.OwningRegion`) "Voyager")
    _
    (elif (`KismetStringLibrary.NotEqual_StrStr` (`self.OwningRegion`))
      (`|ExecutionSequence`
        (:`then_0`
          (bind _result (`BlueprintSetLibrary.Set_ToArray` (`self.ResourceActors`)))
          (for _array_element _result
            (bind _asbp_resource_actor (cast `/Game/Core/BP_ResourceActor` _array_element)
              (:`then`
                (bind _returnvalue (`self.CalculateResourceCollection`))
                (bind _returnvalue_2 (`ResourceActor.ClampAndApplyQuantityChange` _asbp_resource_actor _returnvalue))
                ;[1 1 1] If resource is empty prepare it for removal
                (if (== (`ResourceActor.ResourceQuantity` _asbp_resource_actor) 0)
                  (`BlueprintSetLibrary.Set_Add` (`self.ResourceActorsPendingRemoval`) _asbp_resource_actor))
                (set `self.TotalResourceCollection` (+ _returnvalue_2 (`self.TotalResourceCollection`))))
              (:`CastFailed`
                (`KismetSystemLibrary.PrintString` "Could not cast resource")))))
        (:`then_1`
          (bind _returnvalue_3 (`ResourceManagementSubsystem.IncrementResourceByAmount` (subsystem `ResourceManagementSubsystem`) _owningregion _resourcetype (`self.TotalResourceCollection`)))
          (`KismetSystemLibrary.PrintString` (`KismetStringLibrary.Concat_StrStr` (`KismetStringLibrary.Concat_StrStr` (`KismetStringLibrary.Concat_StrStr` (`KismetStringLibrary.Conv_IntToString` _returnvalue_3) _resourcetype) " total in Region: ") _owningregion))
          (set `self.TotalResourceCollection` 0)
          (`self.RemoveResourceActors`)))
      (else
        (set `self.OwningRegion` (`self.BackupOfOwningRegion`))))))

(fn `RemoveResourceActors`
  (bind _resourceactorspendingremoval (`self.ResourceActorsPendingRemoval`))
  (if (not (== (`BlueprintSetLibrary.Set_Length` _resourceactorspendingremoval) 0))
    (bind _result (`BlueprintSetLibrary.Set_ToArray` _resourceactorspendingremoval))
    (`BlueprintSetLibrary.Set_RemoveItems` (`self.ResourceActors`) _result)
    (for _array_element _result
      (`self.K2_DestroyActor` _array_element))
    (`BlueprintSetLibrary.Set_Clear` (`self.ResourceActorsPendingRemoval`))))

(fn `UserConstructionScript`)