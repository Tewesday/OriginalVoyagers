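; Base unit pawn that travels to a BP_BasicRail path, rides it, and keeps spacing from other units.
; ExecuteInstruction starts a looping timer that moves it toward the path origin with growing steps, halting non-ship units at ocean blockers.
; On arrival it notifies the rail, then snaps to the rail's attachment every Tick until end-of-rail clears the path.
; BubbleCollision overlaps shove other units away, using a Pushing flag to arbitrate.
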(event `MovingToEvent`
  (`self.MoveTo` (stale `self.ExecuteInstruction` _pathorigin)))

(event `self.ExecuteInstruction`
  (bind _pathorigin (`self.GetPathOrigin`))
  (bind _returnvalue (`KismetSystemLibrary.K2_SetTimerDelegate` (delegate `MovingToEvent`) 0.01 true)))

(event `self.ReceiveBeginPlay`
  (add `self.BeginFollowPath` (delegate `StartFollowPath`)))

(event `DoneMovingTo`
  (`KismetSystemLibrary.K2_ClearAndInvalidateTimerHandle` (stale `self.ExecuteInstruction` _returnvalue))
  (`self.FollowPath` :!label _label)
  (`self.SetFollowingPath` true))

(event `StartFollowPath`
  (goto _label))

(event `self.ReceiveTick`
  (params (DeltaSeconds :type "Float (single-precision)"))
  (if (`self.FollowingPath`)
    (`/Engine/EditorBlueprintResources/StandardMacros.IsValid` (`self.Path`)
      (:`Is Valid`
        (`self.FollowPath`)
        (`/Engine/EditorBlueprintResources/StandardMacros.Gate` false :!label _label_2
          (:`Exit`
            (bind _asbp_basic_rail (cast `/Game/Core/BP_BasicRail` (`self.Path`)))
            (add `/Game/Core/BP_BasicRail.EndOfRailReachedEvent` _asbp_basic_rail (delegate `EndOfRail`))
            (goto _label_2 :!via `Close`)))))))

(event `EndOfRail`
  (`self.SetFollowingPath` false)
  (set `self.Path` null)
  (goto _label_2 :!via `Open`))

(event `self.BubbleCollision.OnComponentBeginOverlap`
  (params (OverlappedComponent :type "PrimitiveComponent Object Reference") (OtherActor :type "Actor Object Reference") (OtherComp :type "PrimitiveComponent Object Reference") (OtherBodyIndex :type Integer) (bFromSweep :type Boolean) (SweepResult :type "HitResult Structure (by ref)"))
  (`|ExecutionSequence`
    (:`then_0`
      (if (`KismetMathLibrary.ClassIsChildOf` (`GameplayStatics.GetObjectClass` OtherActor) "BP_UnitPawn_C")
        (bind _asbp_unit_pawn (cast `/Game/Core/BP_UnitPawn` OtherActor))
        (if (!= self _asbp_unit_pawn)
          (set `self.Pushing` true)
          (`self.PushActorAway` _asbp_unit_pawn))))))

(event `self.BubbleCollision.OnComponentEndOverlap`
  (params (OverlappedComponent :type "PrimitiveComponent Object Reference") (OtherActor :type "Actor Object Reference") (OtherComp :type "PrimitiveComponent Object Reference") (OtherBodyIndex :type Integer))
  (bind _overlappingactors (`PrimitiveComponent.GetOverlappingActors` (`self.BubbleCollision`) null))
  (`|ExecutionSequence`
    (:`then_0`
      (if (`KismetMathLibrary.ClassIsChildOf` (`GameplayStatics.GetObjectClass` OtherActor) "BP_UnitPawn_C")
        (set `self.Pushing` false)
        (if (not (== (`KismetArrayLibrary.Array_Length` _overlappingactors) 0))
          (for _array_element _overlappingactors
            (bind _asbp_unit_pawn (cast `/Game/Core/BP_UnitPawn` _array_element))
            (set `self.Pushing` true)
            (`self.PushActorAway` _asbp_unit_pawn)
            (set `self.Pushing` true)))))))

(fn `CallBeginFollowPathEvent`
  (`self.BeginFollowPath`))

(fn `FollowPath`
  (bind _asbp_basic_rail (cast `/Game/Core/BP_BasicRail` (`self.Path`))
    (:`then`
      (`SceneComponent.K2_SetWorldTransform` (`self.Scene`) (`KismetMathLibrary.MakeTransform` (.location (`SceneComponent.K2_GetComponentToWorld` (`/Game/Core/BP_BasicRail.StaticMeshRailAttachment` _asbp_basic_rail)))) false false))
    (:`CastFailed`
      (`KismetSystemLibrary.PrintString` "Fail"))))

(fn `GetPathOrigin`
  (returns (PathOrigin :type "Vector Structure"))
  (bind _returnvalue_location (`KismetMathLibrary.BreakTransform` (`self.GetTransform` (`self.Path`))))
  (return _returnvalue_location))

(fn `GetPushing`
  (returns (PushingResult :type Boolean))
  (return (`self.Pushing`)))

(fn `MoveTo`
  (params (TargetLocation :type "Vector Structure"))
  (locals (HitOcean :type Boolean :default false) (Objects :type "Array of EObjectTypeQuery Enum"))
  (bind _returnvalue (`SceneComponent.K2_GetComponentLocation` (`self.Scene`)))
  (bind _returnvalue_2 (!= TargetLocation _returnvalue :`ErrorTolerance` 30.0))
  (set `local.HitOcean` false)
  (bind _outhits (`KismetSystemLibrary.SphereTraceMultiForObjects` TargetLocation TargetLocation 1.0 (`local.Objects`)))
  (for _array_element _outhits
    (bind _returnvalue_3 (and (!= (`KismetMathLibrary.ClassIsChildOf` (`GameplayStatics.GetObjectClass` self) "/Game/Core/BP_ShipUnitPawn_Child.BP_ShipUnitPawn_Child_C") true) (`KismetMathLibrary.ClassIsChildOf` (`GameplayStatics.GetObjectClass` (`.HitActor` (`GameplayStatics.BreakHitResult` _array_element))) "/Game/Core/BP_OceanBlocker.BP_OceanBlocker_C")))
    (set `local.HitOcean` _returnvalue_3)
    (if _returnvalue_3
      (break)))
  (if (not (`local.HitOcean`))
    (set `self.Alpha` (+ (`self.Alpha`) 0.04))
    (`SceneComponent.K2_SetWorldLocation` (`self.Scene`) (+ (* (`KismetMathLibrary.Normal` (- TargetLocation _returnvalue) 1.0) (`self.Alpha`)) _returnvalue) false false)
    (if _returnvalue_2
      (set `self.MovingTo` _returnvalue_2)
      (else
        (set `self.MovingTo` false)
        (bind _asbp_basic_rail (cast `/Game/Core/BP_BasicRail` (`self.Path`)))
        (`/Game/Core/BP_BasicRail.BeginningOfRailReachedEvent` _asbp_basic_rail)
        (set `self.Alpha` 0.0)
        (`self.DoneMovingTo`)))))

(fn `PushActorAway`
  (params (OtherActor :type "/Game/Core/BP_UnitPawn Object Reference"))
  (bind _location (.location (`self.GetTransform` OtherActor)))
  (if (`self.Pushing`)
    (bind _pushingresult (`self.GetPushing` OtherActor))
    (if _pushingresult
      (set `self.Pushing` false)
      (else
        (`self.K2_SetActorTransform` OtherActor (`KismetMathLibrary.MakeTransform` (- _location (* (`KismetMathLibrary.GetDirectionUnitVector` _location (.location (`self.GetTransform`))) 250.0)) (.rotation (`self.GetTransform` OtherActor)) (.scale (`self.GetTransform` OtherActor))) false false)))))

(fn `SetFollowingPath`
  (params (FollowingPath :type Boolean))
  (set `self.FollowingPath` FollowingPath))

(fn `UserConstructionScript`)