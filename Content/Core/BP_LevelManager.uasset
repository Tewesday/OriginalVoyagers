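; Level manager that registers regions with the resource and population subsystems and seeds structure costs and the first region's starting supplies and units.
; Looping timers drain food by population, wipe starved regions, and show win or loss on the HUD.
; A win requires the temple count to equal the region count; a loss means every region is unpopulated.
; It also registers new Voyager regions and transfers resources and population between regions.
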(event `self.ReceiveBeginPlay`
  (bind _returnvalue (subsystem `ResourceManagementSubsystem`))
  (bind _returnvalue_2 (subsystem `ResourceManagementSubsystem`))
  (bind _regions (`self.Regions`))
  (bind _resourcenames (`ResourceManagementSubsystem.ResourceNames` (subsystem `ResourceManagementSubsystem`)))
  (`|ExecutionSequence`
    (:`then_0`
      (for _ (`ResourceManagementSubsystem.ResourceNames` (subsystem `ResourceManagementSubsystem`))
        _))
    (:`then_1`
      (bind _outactors (`GameplayStatics.GetAllActorsOfClass` "/Game/Core/BP_RegionPawn.BP_RegionPawn_C"))
      (for _array_element _outactors
        (`BlueprintSetLibrary.Set_Add` _regions _array_element))
      (bind _result (`BlueprintSetLibrary.Set_ToArray` _regions))
      ;[1 1 1] Add all regions to ResourceManagementSystem
      (for (_array_element_2 _array_index) _result
        (bind _output_get (set `RegionPawn.RegionName` (`|GetArrayItem` (`self.RegionNames`) _array_index) _array_element_2))
        (`ResourceManagementSubsystem.AddRegion` _returnvalue_2 _output_get)
        ;[1 1 1] Add all regions to Population System
        (`PopulationSubsystem.AddRegion` (subsystem `PopulationSubsystem`) _output_get))
      (`|ExecutionSequence`
        (:`then_0`
          (for _array_element_3 (`self.RegionNames`)
            ;[1 1 1] Add population name default to each region
            (`PopulationSubsystem.AddPopulationName` (subsystem `PopulationSubsystem`) _array_element_3 (`self.PopulationNameDefault`))
            (for _array_element_4 (`ResourceManagementSubsystem.ResourceNames` _returnvalue_2)
              (`ResourceManagementSubsystem.AddResource` _returnvalue_2 _array_element_3 _array_element_4))))))
    (:`then_2`
      (`ResourceManagementSubsystem.AddStructureToCostMap` _returnvalue "WoodCollector" 50)
      (`ResourceManagementSubsystem.AddStructureToCostMap` _returnvalue "FoodCollector" 50)
      (`ResourceManagementSubsystem.AddStructureToCostMap` _returnvalue "CultureCollector" 1000)
      (`ResourceManagementSubsystem.AddStructureToCostMap` _returnvalue "Ship" 300))
    (:`then_3`
      ;[1 1 1] Hardcode 2000 wood for Region1
      (`ResourceManagementSubsystem.IncrementResourceByAmount` _returnvalue (`|GetArrayItem` (`self.RegionNames`)) (`|GetArrayItem` _resourcenames 1) 2000)
      ;[1 1 1] Hardcode 100 Food for Region1
      (`ResourceManagementSubsystem.IncrementResourceByAmount` _returnvalue (`|GetArrayItem` (`self.RegionNames`)) (`|GetArrayItem` _resourcenames) 100))
    (:`then_4`
      ;[1 1 1] Add all starting units to population of starting region
      (bind _outactors_2 (`GameplayStatics.GetAllActorsOfClass` "/Game/Core/BP_UnitPawn.BP_UnitPawn_C"))
      (`PopulationSubsystem.IncrementPopulationByAmount` (subsystem `PopulationSubsystem`) (`|GetArrayItem` (`self.RegionNames`)) (`self.PopulationNameDefault`) (`KismetArrayLibrary.Array_Length` _outactors_2)))
    (:`then_5`
      (`KismetSystemLibrary.K2_SetTimer` null "FoodDecay" 10.0 true))
    (:`then_6`
      (`|ExecutionSequence`
        (:`then_0`
          (`KismetSystemLibrary.K2_SetTimer` null "CheckWinCondition" 3.8 true))
        (:`then_1`
          (`KismetSystemLibrary.K2_SetTimer` null "CheckFoodWithPop" 5.8 true))
        (:`then_2`
          (`KismetSystemLibrary.K2_SetTimer` null "CheckLossCondition" 6.3 true))))))

(fn `AddNewRegion`
  (params (NewRegion :type "/Game/Core/BP_RegionPawn Object Reference"))
  (bind _returnvalue (subsystem `ResourceManagementSubsystem`))
  (bind _returnvalue_2 (subsystem `PopulationSubsystem`))
  (bind _regionnames (`self.RegionNames`))
  ;[1 1 1] Add to LevelManager
  (`BlueprintSetLibrary.Set_Add` (`self.Regions`) NewRegion)
  (bind _output_get (set `RegionPawn.RegionName` (`KismetStringLibrary.Concat_StrStr` "Voyager" (`KismetStringLibrary.Conv_IntToString` (+ (`KismetArrayLibrary.Array_Length` _regionnames) 1))) NewRegion))
  (`KismetArrayLibrary.Array_Add` _regionnames _output_get)
  ;[1 1 1] Add to Systems
  (`ResourceManagementSubsystem.AddRegion` _returnvalue _output_get)
  (`PopulationSubsystem.AddRegion` _returnvalue_2 _output_get)
  (`PopulationSubsystem.AddPopulationName` _returnvalue_2 _output_get (`self.PopulationNameDefault`))
  (for _array_element (`ResourceManagementSubsystem.ResourceNames` _returnvalue)
    (`ResourceManagementSubsystem.AddResource` _returnvalue _output_get _array_element)))

(fn `AddPopulation`)

(fn `CheckFoodWithPop`
  (bind _returnvalue (subsystem `PopulationSubsystem`))
  (for _array_element (`self.RegionNames`)
    (bind _returnvalue_2 (`ResourceManagementSubsystem.RetrieveResourceValue` (subsystem `ResourceManagementSubsystem`) _array_element "Food"))
    (bind _returnvalue_3 (`PopulationSubsystem.RetrievePopulationValue` _returnvalue _array_element (`self.PopulationNameDefault`)))
    ;[1 1 1] If any region has no food but has population, remove population there
    (if (and (== _returnvalue_2 0) (!= _returnvalue_3 0))
      (bind _result (`BlueprintSetLibrary.Set_ToArray` (`self.Regions`)))
      (for _array_element_2 _result
        (if (`KismetStringLibrary.EqualEqual_StrStr` _array_element (`RegionPawn.RegionName` _array_element_2))
          (`/Game/Core/BP_RegionPawn.DespawnUnitsInRegion` _array_element_2 10000)
          (`PopulationSubsystem.DecrementPopulationByAmount` _returnvalue _array_element (`self.PopulationNameDefault`) 10000))))))

(fn `CheckLossCondition`
  (locals (RegionsWithoutPopulation :type Integer))
  (bind _regionnames (`self.RegionNames`))
  (set `local.RegionsWithoutPopulation` 0)
  (for _array_element _regionnames
    (bind _returnvalue (`PopulationSubsystem.RetrievePopulationValue` (subsystem `PopulationSubsystem`) _array_element (`self.PopulationNameDefault`)))
    (if (== _returnvalue 0)
      (`/Engine/EditorBlueprintResources/StandardMacros.IncrementInt` (`local.RegionsWithoutPopulation`))))
  ;[1 1 1] If all regions have no population, player loss
  (if (== (`KismetArrayLibrary.Array_Length` _regionnames) (`local.RegionsWithoutPopulation`))
    (bind _asbp_basic_hud (cast `/Game/Core/BP_BasicHUD` (`PlayerController.GetHUD` (`GameplayStatics.GetPlayerController` 0))))
    (`/Game/Core/BP_BasicHUD.DisplayLoss` _asbp_basic_hud)))

(fn `CheckWinCondition`
  (locals (NumberOfTemples :type Integer))
  (bind _result (`BlueprintSetLibrary.Set_ToArray` (`self.Regions`)))
  (for _array_element _result
    (bind _result_2 (`BlueprintSetLibrary.Set_ToArray` (`/Game/Core/BP_RegionPawn.StructuresInRegion` _array_element)))
    (for _array_element_2 _result_2
      (if (`KismetMathLibrary.ClassIsChildOf` (`GameplayStatics.GetObjectClass` _array_element_2) "/Game/Core/BP_PopulationStructureActor_Child.BP_PopulationStructureActor_Child_C")
        (`/Engine/EditorBlueprintResources/StandardMacros.IncrementInt` (`local.NumberOfTemples`)))))
  ;[1 1 1] Number of temples = number of regions = win
  (if (== (`KismetArrayLibrary.Array_Length` _result) (`local.NumberOfTemples`))
    (bind _asbp_basic_hud (cast `/Game/Core/BP_BasicHUD` (`PlayerController.GetHUD` (`GameplayStatics.GetPlayerController` 0))))
    (`/Game/Core/BP_BasicHUD.DisplayWin` _asbp_basic_hud)))

(fn `FoodDecay`
  (locals (DecayMultiplier :type Integer :default 1))
  (bind _returnvalue (subsystem `ResourceManagementSubsystem`))
  (for _array_element (`self.RegionNames`)
    (bind _returnvalue_2 (`PopulationSubsystem.RetrievePopulationValue` (subsystem `PopulationSubsystem`) _array_element (`self.PopulationNameDefault`)))
    (bind _returnvalue_3 (* _returnvalue_2 (`local.DecayMultiplier`)))
    (`ResourceManagementSubsystem.DecrementResourceByAmount` _returnvalue _array_element (`|GetArrayItem` (`ResourceManagementSubsystem.ResourceNames` _returnvalue)) _returnvalue_3)
    (`KismetSystemLibrary.PrintString` (`KismetStringLibrary.Concat_StrStr` (`KismetStringLibrary.Conv_IntToString` _returnvalue_3) " Food lost due to pop"))))

(fn `GetRegionUsingName`
  (params (RegionName :type String))
  (returns (RegionChosen :type "/Game/Core/BP_RegionPawn Object Reference"))
  (locals (RegionChosenFromLoop :type "/Game/Core/BP_RegionPawn Object Reference"))
  (bind _result (`BlueprintSetLibrary.Set_ToArray` (`self.Regions`)))
  (for _array_element _result
    (if (`KismetStringLibrary.EqualEqual_StrStr` RegionName (`RegionPawn.RegionName` _array_element))
      (set `local.RegionChosenFromLoop` _array_element)))
  (return (`local.RegionChosenFromLoop`)))

(fn `TransferPopulationBetweenRegions`
  (params (DesiredWeightOfRegionTo :type Integer) (RegionTo :type String) (AmountToTransfer :type Integer))
  (bind _currentlyselectedregion (`self.CurrentlySelectedRegion`))
  (bind _returnvalue (`PopulationSubsystem.TransferPopulationByAmount` (subsystem `PopulationSubsystem`) _currentlyselectedregion RegionTo (`self.PopulationNameDefault`) AmountToTransfer))
  (`|ExecutionSequence`
    (:`then_0`
      ;[1 1 1] Tell region from to despawn units
      (bind _regionchosen (`self.GetRegionUsingName` _currentlyselectedregion))
      (if (`/Game/Core/BP_RegionPawn.IsAnIsland` _regionchosen)
        (`/Game/Core/BP_RegionPawn.DespawnUnitsInRegion` _regionchosen AmountToTransfer)))
    (:`then_1`
      ;[1 1 1] If region from is a boat, then tell it to spawn units for next region
      (bind _regionchosen_2 (`self.GetRegionUsingName` _currentlyselectedregion))
      (if (not (`/Game/Core/BP_RegionPawn.IsAnIsland` _regionchosen_2))
        (`/Game/Core/BP_ShipUnitPawn_Child.SpawnPopulationAsUnits` (`/Game/Core/BP_RegionPawn.OwningShip` _regionchosen_2) _returnvalue)))))

(fn `TransferResourcesBetweenRegions`
  (params (DesiredWeightOfRegionTo :type Integer) (RegionTo :type String) (ResourcesToTransfer :type "Array of String") (AmountToTransfer :type "Array of Integer"))
  (bind _regionchosen (`self.GetRegionUsingName` RegionTo))
  (if (>= (`/Game/Core/BP_RegionPawn.RegionMaxWeight` _regionchosen) DesiredWeightOfRegionTo)
    ;[1 1 1] Set weight of target region
    (bind _regionchosen_2 (`self.GetRegionUsingName` RegionTo))
    (set `/Game/Core/BP_RegionPawn.RegionCurrentWeight` DesiredWeightOfRegionTo _regionchosen_2)
    ;[1 1 1] Transfer each resource from region to region
    (for (_array_element _array_index) ResourcesToTransfer
      (`ResourceManagementSubsystem.TransferResourceByAmount` (subsystem `ResourceManagementSubsystem`) (`self.CurrentlySelectedRegion`) RegionTo _array_element (`|GetArrayItem` AmountToTransfer _array_index)))))

(fn `UserConstructionScript`)