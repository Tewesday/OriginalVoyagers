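; Child ship pawn that carries its own region, so the ship acts as a mobile, non-island region.
; On BeginPlay it spawns a BP_RegionPawn with an enlarged box, sets its max weight and owning ship, and registers it with every BP_LevelManager.
; Tick moves the region's scene component to the ship's location.
; SpawnPopulationAsUnits spawns BP_UnitPawns in a diagonal line from the ship at zero height until the requested count is reached.
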(event `self.ReceiveBeginPlay`
  (`parent.ReceiveBeginPlay`)
  (bind _returnvalue (`|SpawnActorFromClass` "/Game/Core/BP_RegionPawn.BP_RegionPawn_C" (`self.GetTransform`) "AlwaysSpawn" "OverrideRootScale" null null))
  (bind _output_get (set `self.RegionOfShip` _returnvalue))
  (`SceneComponent.SetWorldScale3D` (`self.GetComponentByClass` _returnvalue "/Script/Engine.BoxComponent") (80.0 80.0 5.0))
  (set `/Game/Core/BP_RegionPawn.RegionMaxWeight` 200 _output_get)
  (set `/Game/Core/BP_RegionPawn.IsAnIsland` false _returnvalue)
  (set `/Game/Core/BP_RegionPawn.OwningShip` self _returnvalue)
  (bind _outactors (`GameplayStatics.GetAllActorsOfClass` "/Game/Core/BP_LevelManager.BP_LevelManager_C"))
  (for _array_element _outactors
    (`/Game/Core/BP_LevelManager.AddNewRegion` _array_element _output_get)))

(event `self.ReceiveTick`
  (params (DeltaSeconds :type "Float (single-precision)"))
  (`parent.ReceiveTick` DeltaSeconds)
  (`SceneComponent.K2_SetWorldLocation` (`/Game/Core/BP_RegionPawn.Scene` (`self.RegionOfShip`)) (.location (`self.GetTransform`)) false false))

(fn `SpawnPopulationAsUnits`
  (params (PopulationNumber :type Integer))
  (locals (CurrentlySpawnedUnits :type Integer) (DistanceMultiplier :type "Float (double-precision)" :default 1000.0))
  (bind _currentlyspawnedunits (`local.CurrentlySpawnedUnits`))
  (bind _returnvalue (* (+ _currentlyspawnedunits 1) (`local.DistanceMultiplier`)))
  (while (!= _currentlyspawnedunits PopulationNumber)
    (`|SpawnActorFromClass` "/Game/Core/BP_UnitPawn.BP_UnitPawn_C" (`KismetMathLibrary.MakeTransform` (`KismetMathLibrary.MakeVector` (+ _returnvalue (.x (.location (`self.GetTransform`)))) (+ _returnvalue (.y (.location (`self.GetTransform`)))))) "AlwaysSpawn" "OverrideRootScale" null null)
    (`/Engine/EditorBlueprintResources/StandardMacros.IncrementInt` (`local.CurrentlySpawnedUnits`))))

(fn `UserConstructionScript`
  (`parent.UserConstructionScript`))